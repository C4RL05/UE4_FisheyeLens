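; HUD Blueprint that marks an Objective actor's screen position with and without fisheye distortion.
; DrawHUD projects the actor to screen, drawing a small red square at the raw point and a green one at the distorted point.
; The Fisheye function converts pixels to clamped UV, applies a UV-space Fisheye call using angle and view size, then scales back to pixels.
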(event EventDrawHUD
  (params (SizeX :type Integer) (SizeY :type Integer))
  (bind _objective (Variables|Default|GetObjective)
    (:then
      (HUD|DrawRect "(R=1.000000,G=0.000000,B=0.000000,A=1.000000)" (.X (Math|Vector2D|BreakVector2D (- (.ScreenLocation (Class|PlayerController|ProjectWorldLocationtoScreen (Game|GetPlayerController 0) (Transformation|GetActorLocation _objective) false)) 4.0))) (.Y (Math|Vector2D|BreakVector2D (- (.ScreenLocation (Class|PlayerController|ProjectWorldLocationtoScreen (Game|GetPlayerController 0) (Transformation|GetActorLocation _objective) false)) 4.0))) 8.0 8.0)
      (bind _outlocation (CallFunction|Fisheye (.ScreenLocation (Class|PlayerController|ProjectWorldLocationtoScreen (Game|GetPlayerController 0) (Transformation|GetActorLocation _objective) false)) -2.0 (Math|Vector2D|MakeVector2D (Math|Conversions|ToFloat(Integer) SizeX) (Math|Conversions|ToFloat(Integer) SizeY))))
      (HUD|DrawRect "(R=0.000000,G=1.000000,B=0.000000,A=1.000000)" (.X (Math|Vector2D|BreakVector2D (- _outlocation 4.0))) (.Y (Math|Vector2D|BreakVector2D (- _outlocation 4.0))) 8.0 8.0))
    (:else)))

(fn ConstructionScript)

(fn Fisheye
  (params (InLocation :type Vector%202D%20Structure) (Angle :type Float%20%28single-precision%29) (ViewSize :type Vector%202D%20Structure))
  (return (* (CallFunction|Fisheye (Class|KismetMathLibrary|ClampAxes2D (/ InLocation ViewSize) 0.0 1.0) ViewSize Angle) ViewSize)))